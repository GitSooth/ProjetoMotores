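; Player soldier character Blueprint with camera-relative movement, jumping, sprinting, aiming and shooting.
; Aiming toggles the HUD crosshair, narrows camera FOV, switches rotation to follow the controller and blocks jumping and starting a sprint.
; Firing line-traces from the camera with persistent debug drawing and destroys hit actors tagged Enemy.
; Only for such hits that also cast to ThirdPersonCharacter, a Bullet spawns at the muzzle socket facing the impact point.
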(event `InputAxis|MoveForward`
  (params (AxisValue :type "Float (single-precision)"))
  ;[1 1 1] Movement
  (`self.AddMovementInput` (`KismetMathLibrary.GetForwardVector` (`KismetMathLibrary.MakeRotator` 0.0 0.0 (.yaw (`self.GetControlRotation`)))) AxisValue))

(event `InputAction|Jump`
  (params (Key :type "Key Structure"))
  ;[1 1 1] Movement
  (:`Pressed`
    (set `self.isJumping` true)
    (if (not (`self.isAiming`))
      (`self.Jump`)))
  (:`Released`
    (set `self.isJumping` false)))

(event `InputAxis|MoveRight`
  (params (AxisValue :type "Float (single-precision)"))
  ;[1 1 1] Movement
  (`self.AddMovementInput` (`KismetMathLibrary.GetRightVector` (`KismetMathLibrary.MakeRotator` 0.0 0.0 (.yaw (`self.GetControlRotation`)))) AxisValue))

(event `InputAxis|Turn`
  (params (AxisValue :type "Float (single-precision)"))
  ;[1 1 1] Movement
  (`self.AddControllerYawInput` AxisValue))

(event `InputAction|ToggleAim`
  (params (Key :type "Key Structure"))
  (bind _camera (`self.Camera`))
  (bind _charactermovement (`self.CharacterMovement`))
  (bind _returnvalue (`PlayerController.GetHUD` (`GameplayStatics.GetPlayerController` 0)))
  ;[1 1 1] Movement
  (:`Pressed`
    (set `self.isAiming` true)
    (message `/Game/Assets/UI/BPI_UI.ToggleCrosshair` _returnvalue true)
    (`CameraComponent.SetFieldOfView` _camera 70.0)
    (set `CharacterMovementComponent.bOrientRotationToMovement` false _charactermovement)
    (set `CharacterMovementComponent.bUseControllerDesiredRotation` true _charactermovement))
  (:`Released`
    (set `self.isAiming` false)
    (message `/Game/Assets/UI/BPI_UI.ToggleCrosshair` _returnvalue false)
    (`CameraComponent.SetFieldOfView` _camera 90.0)
    (set `CharacterMovementComponent.bOrientRotationToMovement` true _charactermovement)
    (set `CharacterMovementComponent.bUseControllerDesiredRotation` false _charactermovement)))

(event `Key|LeftShift`
  (params (Key :type "Key Structure"))
  (bind _charactermovement (`self.CharacterMovement`))
  ;[1 1 1] Movement
  (:`Pressed`
    (if (not (`self.isAiming`))
      (set `CharacterMovementComponent.MaxWalkSpeed` 600.0 _charactermovement)))
  (:`Released`
    (set `CharacterMovementComponent.MaxWalkSpeed` 300.0 _charactermovement)))

(event `InputAxis|LookUp`
  (params (AxisValue :type "Float (single-precision)"))
  ;[1 1 1] Movement
  (`self.AddControllerPitchInput` AxisValue))

(event `InputAction|Fire`
  (params (Key :type "Key Structure"))
  (bind _camera (`self.Camera`))
  (bind _returnvalue (`SceneComponent.K2_GetComponentLocation` _camera))
  (bind _returnvalue_2 (`SceneComponent.GetSocketLocation` (`self.SK_AR4`) "b_gun_muzzleflash"))
  (:`Pressed`
    (set `self.isShooting` true)
    (bind (_outhit _returnvalue_3) (`KismetSystemLibrary.LineTraceSingle` :`Start` _returnvalue :`End` (+ (* (`SceneComponent.GetForwardVector` _camera) 5000.0) _returnvalue) :`TraceChannel` "TraceTypeQuery1" :`DrawDebugType` "Persistent"))
    (bind (_bblockinghit _binitialoverlap _time _distance _location _impactpoint _normal _impactnormal _physmat _hitactor _hitcomponent _hitbonename _hititem _elementindex _faceindex _tracestart _traceend) (`GameplayStatics.BreakHitResult` _outhit))
    (`/Engine/EditorBlueprintResources/StandardMacros.IsValid` _hitactor
      (:`Is Valid`
        (if (`self.ActorHasTag` _hitactor "Enemy")
          (`self.K2_DestroyActor` _hitactor)
          (cast `/Game/ThirdPersonBP/Blueprints/ThirdPersonCharacter` _hitactor)
          (`|SpawnActorFromClass` "/Game/Assets/Character/Bullet.Bullet_C" (`KismetMathLibrary.MakeTransform` _returnvalue_2 (`KismetMathLibrary.FindLookAtRotation` _returnvalue_2 (`KismetMathLibrary.SelectVector` _impactpoint _traceend _returnvalue_3))) "Undefined" "OverrideRootScale" null null)))))
  (:`Released`
    (set `self.isShooting` false)))

(fn `UserConstructionScript`)