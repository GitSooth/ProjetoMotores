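; LaunchPad_BP is a launch pad actor that throws the player character when they step into its Box trigger.
; On overlap, it checks for player 0 and calls LaunchCharacter along the Arrow component's forward vector scaled by LaunchForce, with configurable XY and Z override flags.
; It then casts the player to SoldierBP and sets IsJumping to true.
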(event `self.Box.OnComponentBeginOverlap`
  (params (OverlappedComponent :type "PrimitiveComponent Object Reference") (OtherActor :type "Actor Object Reference") (OtherComp :type "PrimitiveComponent Object Reference") (OtherBodyIndex :type Integer) (bFromSweep :type Boolean) (SweepResult :type "HitResult Structure (by ref)"))
  (bind _returnvalue (`GameplayStatics.GetPlayerCharacter` 0))
  ;[1 1 1] Confirms if its the player and Launches him into the air
  (if (== OtherActor _returnvalue)
    (`Character.LaunchCharacter` _returnvalue (* (`SceneComponent.GetForwardVector` (`self.Arrow`)) (`self.LaunchForce`)) (`self.XYOverride`) (`self.ZOverride`))
    (bind _assoldier_bp (cast `/Game/Assets/Character/SoldierBP` _returnvalue))
    (set `/Game/Assets/Character/SoldierBP.isJumping` true _assoldier_bp)))

(fn `UserConstructionScript`)