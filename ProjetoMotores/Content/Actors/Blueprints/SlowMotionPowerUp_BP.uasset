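; Slow-motion power-up pickup that halves global time dilation when the player pawn overlaps its Box.
; The pickup toggles the Cube's visibility and uses a CanColide flag to block retriggering while the effect runs.
; After a Delay, which runs in dilated game time, it restores normal speed, toggles the Cube back and re-arms itself for reuse.
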(event `self.Box.OnComponentBeginOverlap`
  (params (OverlappedComponent :type "PrimitiveComponent Object Reference") (OtherActor :type "Actor Object Reference") (OtherComp :type "PrimitiveComponent Object Reference") (OtherBodyIndex :type Integer) (bFromSweep :type Boolean) (SweepResult :type "HitResult Structure (by ref)"))
  (bind _cube (`self.Cube`))
  (if (== OtherActor (`GameplayStatics.GetPlayerPawn` 0))
    (if (`self.CanColide`)
      (`SceneComponent.ToggleVisibility` _cube true)
      (set `self.CanColide` false)
      (`GameplayStatics.SetGlobalTimeDilation` 0.5)
      (`KismetSystemLibrary.Delay` 2.5)
      (`GameplayStatics.SetGlobalTimeDilation` 1.0)
      (`SceneComponent.ToggleVisibility` _cube false)
      (set `self.CanColide` true))))

(fn `UserConstructionScript`)