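; MovingTarget_BP is a target actor that slides back and forth along its Y axis around its starting position.
; BeginPlay stores the root component's starting location, and Tick flips the MoveLeft flag whenever the actor passes MovementRange on either side.
; MoveTarget offsets the root's relative Y by direction times Speed each frame without sweep or delta-time scaling, so movement speed depends on frame rate.
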(event `self.ReceiveBeginPlay`
  (set `self.StartingLocation` (`SceneComponent.RelativeLocation` (`self.DefaultSceneRoot`))))

(event `self.ReceiveTick`
  (params (DeltaSeconds :type "Float (single-precision)"))
  (bind (_startinglocation_x _startinglocation_y) (`KismetMathLibrary.BreakVector` (`self.StartingLocation`)))
  (bind _movementrange (`self.MovementRange`))
  (bind (_relativelocation_x _relativelocation_y) (`KismetMathLibrary.BreakVector` (`SceneComponent.RelativeLocation` (`self.DefaultSceneRoot`))))
  (if (`self.MoveLeft`)
    (if (< _relativelocation_y (+ _startinglocation_y _movementrange))
      (set `self.MovementDirection` 10.0)
      (`self.MoveTarget`)
      (else
        (set `self.MoveLeft` false)))
    (elif (> _relativelocation_y (- _startinglocation_y _movementrange))
      (set `self.MovementDirection` -10.0)
      (`self.MoveTarget`)
      (else
        (set `self.MoveLeft` true)))))

(fn `MoveTarget`
  (bind _defaultsceneroot (`self.DefaultSceneRoot`))
  (bind (_relativelocation_x _relativelocation_y _relativelocation_z) (`KismetMathLibrary.BreakVector` (`SceneComponent.RelativeLocation` _defaultsceneroot)))
  (`SceneComponent.K2_SetRelativeLocation` _defaultsceneroot (`KismetMathLibrary.MakeVector` _relativelocation_x (+ (* (`self.MovementDirection`) (`self.Speed`)) _relativelocation_y) _relativelocation_z) false false))

(fn `UserConstructionScript`)